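; Player-controllable tank Blueprint that connects input to track movement, camera aiming and firing.
; On BeginPlay it hands both tracks to TankNavMovement and the barrel and turret to TankAiming.
; Aim axes rotate the azimuth gimbal and spring arm separately, and FirePrimary calls Fire.
; Driving works either through direct per-track throttles or through forward and turn intents sent to TankNavMovement.
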(event EventBeginPlay
  (Class|TankNavMovementComponent|Initialize (Variables|Default|GetTankNavMovement) (Variables|Default|GetLeftTrack) (Variables|Default|GetRightTrack))
  (Class|TankAimingComponent|Initialize (Variables|Default|GetTankAiming) (Variables|Default|GetTankBarrel) (Variables|Default|GetTankTurret)))

(event Collision|EventActorBeginOverlap
  (params (OtherActor :type Actor%20Object%20Reference)))

(event EventTick
  (params (DeltaSeconds :type Float%20%28single-precision%29)))

(event Input|ActionEvents|InputActionFirePrimary
  (params (Key :type Key%20Structure))
  (:Pressed
    (Class|Tank|Fire)))

(event Input|AxisEvents|InputAxisAimAzimuth
  (params (AxisValue :type Float%20%28single-precision%29))
  ;[1 1 1] Aim Input Control
  (Transformation|AddLocalRotation (Variables|Default|GetAzimuth%20Gimbal) (Math|Rotator|MakeRotator 0.0 0.0 AxisValue) false false))

(event Input|AxisEvents|InputAxisAimElevation
  (params (AxisValue :type Float%20%28single-precision%29))
  ;[1 1 1] Aim Input Control
  (Transformation|AddLocalRotation (Variables|Default|GetSpringArm) (Math|Rotator|MakeRotator 0.0 AxisValue 0.0) false false))

(event Input|AxisEvents|InputAxisLeftTrackThrottle
  (params (AxisValue :type Float%20%28single-precision%29))
  ;[1 1 1] Movement Input Control
  (Class|TankTrackComponent|SetThrottle (Variables|Default|GetLeftTrack) AxisValue))

(event Input|AxisEvents|InputAxisRightTrackThrottle
  (params (AxisValue :type Float%20%28single-precision%29))
  ;[1 1 1] Movement Input Control
  (Class|TankTrackComponent|SetThrottle (Variables|Default|GetRightTrack) AxisValue))

(event Input|AxisEvents|InputAxisThrottleY
  (params (AxisValue :type Float%20%28single-precision%29))
  ;[1 1 1] Movement Input Control
  (Class|TankNavMovementComponent|IntendMoveForward (Variables|Default|GetTankNavMovement) AxisValue))

(event Input|AxisEvents|InputAxisThrottleX
  (params (AxisValue :type Float%20%28single-precision%29))
  ;[1 1 1] Movement Input Control
  (Class|TankNavMovementComponent|IntendTurn (Variables|Default|GetTankNavMovement) AxisValue))

(fn ConstructionScript)